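; Door actor meant to open on an E press by hiding its two cubes and disabling collision on one.
; When BP_ShooterCharacter leaves the overlap, it restores visibility and collision and disables the actor's input.
; On overlap begin, enabling input and hiding a third cube sit behind a branch fixed to false, so neither runs and no key check is present.
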(event Collision|EventActorBeginOverlap
  (params (OtherActor :type Actor%20Object%20Reference))
  (Utilities|Casting|CastToBP_ShooterCharacter OtherActor)
  (if false
    (Input|EnableInput (Game|GetPlayerController 0))
    (Rendering|SetVisibility (Variables|Default|GetCube2) false false)))

(event Collision|EventActorEndOverlap
  (params (OtherActor :type Actor%20Object%20Reference))
  (Utilities|Casting|CastToBP_ShooterCharacter OtherActor)
  (Rendering|SetVisibility (Variables|Default|GetCube1) true false)
  (Collision|SetCollisionEnabled (Variables|Default|GetCube) "QueryAndPhysics")
  (Input|DisableInput (Game|GetPlayerController 0)))

(event Input|KeyboardEvents|E
  (params (Key :type Key%20Structure :default "None"))
  (:Pressed
    (Rendering|SetVisibility (Variables|Default|GetCube1) false false)
    (Collision|SetCollisionEnabled (Variables|Default|GetCube) "NoCollision")))

(fn ConstructionScript)